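; Audio-reactive spotlight actor that shifts color with one frequency band of the music.
; Shortly after BeginPlay it binds to the player BP_ThirdPersonCharacter's OnMusicPlaying dispatcher.
; Each update blends the light between MinColor and MaxColor by the BandToViz value, and can print tracked min/max levels for debugging.
; It also computes a target pitch, but the interpolated rotation logic is disconnected from Tick.
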(event Custom|OnMusicPlaying_Event
  (params (Bands :type Array%20of%20Floats%20%28double-precision%29))
  (bind _bandtoviz (Variables|Default|GetBandToViz))
  (bind _output (Utilities|Array|Get(acopy) Bands _bandtoviz))
  (CallFunction|SetMinMaxValues _output (Variables|Default|GetShow%20Min%20Max%20Values))
  (Rendering|Components|Light|SetLightColor (Variables|Default|GetSpotLight) (Math|Color|Lerp(LinearColor) (Variables|Default|GetMinColor) (Variables|Default|GetMaxColor) (Math|Float|MapRangeClamped _output 0.0 1.0 0.0 1.0)) true)
  (Variables|Default|SetNewRotation (Math|Float|MapRangeClamped _output 0.0 1.0 0.0 3e+01)))

(event EventBeginPlay
  (Utilities|FlowControl|Delay 2.0)
  (bind _asbp_third_person_character (Utilities|Casting|CastToBP_ThirdPersonCharacter (Game|Player|GetPlayerPawn 0)))
  (EventDispatchers|AssignOnMusicPlaying _asbp_third_person_character (delegate Custom|OnMusicPlaying_Event)))

(event EventTick
  (params (DeltaSeconds :type Float%20%28single-precision%29)))

(fn ConstructionScript
  (Rendering|Components|Light|SetLightColor (Variables|Default|GetSpotLight) (Variables|Default|GetMinColor) true))

(fn SetMinMaxValues
  (params (Value :type Float%20%28double-precision%29) (bShowMinMaxValues :type Boolean))
  (Variables|Default|SetMin (Math|Float|SelectFloat Value (Variables|Default|GetMin) (< Value (Variables|Default|GetMin))))
  (Variables|Default|SetMax (Math|Float|SelectFloat Value (Variables|Default|GetMax) (> Value (Variables|Default|GetMax))))
  (if bShowMinMaxValues
    (Development|PrintString (Utilities|String|ToString(Float) (Variables|Default|Getmax)) true false "(R=1.000000,G=0.030401,B=0.000000,A=1.000000)" 0.0 "Max")
    (Development|PrintString (Utilities|String|ToString(Float) (Variables|Default|Getmin)) true false "(R=0.000000,G=1.000000,B=0.064858,A=1.000000)" 0.0 "Min")
    (Development|PrintString (Utilities|String|ToString(Float) Value) true false "(R=0.000000,G=0.216044,B=1.000000,A=1.000000)" 0.0 "Value")))