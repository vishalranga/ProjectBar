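; Audio visualizer actor that recolors a row of spotlights to match the spectrum of playing music.
; The construction script spawns one spotlight and index text label per band in NRTSettings, spaced by Padding.
; Two seconds after BeginPlay it binds to the third-person character's OnMusicPlaying event, lerping each light between MinColor and MaxColor by its band value.
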(event Custom|OnMusicPlaying_Event
  (params (Bands :type Array%20of%20Floats%20%28double-precision%29))
  (for (_array_element _array_index) (Variables|Default|GetMeshComponents)
    (Rendering|Components|Light|SetLightColor _array_element (Math|Color|Lerp(LinearColor) (Variables|Default|GetMinColor) (Variables|Default|GetMaxColor) (Math|Float|MapRangeClamped (Utilities|Array|Get(acopy) Bands _array_index) 0.0 1.0 0.0 1.25)) true)))

(event EventBeginPlay
  (Utilities|FlowControl|Delay 2.0)
  (bind _asbp_third_person_character (Utilities|Casting|CastToBP_ThirdPersonCharacter (Game|Player|GetPlayerPawn 0)))
  (EventDispatchers|AssignOnMusicPlaying _asbp_third_person_character (delegate Custom|OnMusicPlaying_Event)))

(fn ConstructionScript
  (CallFunction|GenerateBandMeshes))

(fn GenerateBandMeshes
  (Utilities|Array|Clear (Variables|Default|GetMeshComponents))
  (for _index (range 0 (- (Variables|/Script/AudioSynesthesia.ConstantQNRTSettings|GetNumBands (Variables|Default|GetNRT_Settings)) 1))
    (bind _returnvalue (AddComponent|AddTextRenderComponent false (Math|Transform|MakeTransform (Math|Vector|MakeVector (* (Variables|Default|GetPadding) _index) -1e+02 0.0) "90.000000,0.000000,-90.000000")))
    (Rendering|Components|TextRender|SetText _returnvalue (Utilities|Text|ToText(Integer) _index))
    (bind _returnvalue_2 (AddComponent|AddSpotLightComponent false (Math|Transform|MakeTransform (Math|Vector|MakeVector (* (Variables|Default|GetPadding) _index) 0.0 0.0) (Variables|Default|GetRotation))))
    (Utilities|Array|Add (Variables|Default|GetMeshComponents) _returnvalue_2)
    (Rendering|Components|Light|SetLightColor _returnvalue_2 (Variables|Default|GetMinColor) true)))