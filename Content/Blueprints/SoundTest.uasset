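; SoundTest is a music visualizer actor that drives a spotlight from one selectable audio band.
; After a short delay following BeginPlay, it binds to the player ThirdPerson character's OnMusicPlaying dispatcher.
; Each broadcast maps the chosen band's value to a blend between two colors and a target angle.
; Tick smoothly interpolates the light's pitch toward that angle.
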(event Custom|OnMusicPlaying_Event
  (params (Bands :type Array%20of%20Floats%20%28double-precision%29))
  (bind _bandtoviz (Variables|Default|GetBandToViz))
  (bind _output (Utilities|Array|Get(acopy) Bands _bandtoviz))
  (Rendering|Components|Light|SetLightColor (Variables|Default|GetSpotLight) (Math|Conversions|ToLinearColor(Vector) (Math|Vector|Lerp(Vector) (Variables|Default|GetB) (Variables|Default|GetA) (Math|Float|MapRangeClamped _output 0.0 1.0 0.0 5.0))) true)
  (Variables|Default|SetNewRotation (Math|Float|MapRangeClamped _output 0.0 1.0 0.0 3e+01)))

(event EventBeginPlay
  (Utilities|FlowControl|Delay 2.0)
  (bind _asbp_third_person_character (Utilities|Casting|CastToBP_ThirdPersonCharacter (Game|Player|GetPlayerPawn 0)))
  (EventDispatchers|AssignOnMusicPlaying _asbp_third_person_character (delegate Custom|OnMusicPlaying_Event)))

(event EventTick
  (params (DeltaSeconds :type Float%20%28single-precision%29))
  (Transformation|SetRelativeRotation (Variables|Default|GetSpotLight) (Math|Rotator|MakeRotator 0.0 (Math|Interpolation|FInterpTo (.pitch (Variables|/Script/Engine.SceneComponent|GetRelativeRotation (Variables|Default|GetSpotLight))) (Variables|Default|GetNewRotation) DeltaSeconds 2e+01) 0.0) false false))

(fn ConstructionScript)