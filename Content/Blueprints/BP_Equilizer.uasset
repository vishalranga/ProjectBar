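; Music equalizer actor that visualizes frequency bands as a row of glowing meshes.
; The construction script spawns one mesh per band in the Constant-Q NRT settings, spaced along X, each with a random emissive color from Colors.
; After a short BeginPlay delay, it binds to the third-person character's OnMusicPlaying dispatcher.
; Each broadcast remaps band values into the matching mesh's Y scale.
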(event Custom|OnMusicPlaying_Event
  (params (Bands :type Array%20of%20Floats%20%28double-precision%29))
  (bind _scale (Variables|Default|GetScale))
  (for (_array_element _array_index) (Variables|Default|GetMeshComponents)
    (Transformation|SetRelativeScale3D _array_element (Math|Vector|MakeVector (.x _scale) (Math|Float|MapRangeClamped (Utilities|Array|Get(acopy) Bands _array_index) -31.0 13.0 0.0 3.0) (.z _scale)))))

(event EventBeginPlay
  (Utilities|FlowControl|Delay 2.0)
  (bind _asbp_third_person_character (Utilities|Casting|CastToBP_ThirdPersonCharacter (Game|Player|GetPlayerPawn 0)))
  (EventDispatchers|AssignOnMusicPlaying _asbp_third_person_character (delegate Custom|OnMusicPlaying_Event)))

(fn ConstructionScript
  (CallFunction|GenerateBandMeshes))

(fn GenerateBandMeshes
  (Utilities|Array|Clear (Variables|Default|GetMeshComponents))
  (for _index (range 0 (- (Variables|/Script/AudioSynesthesia.ConstantQNRTSettings|GetNumBands (Variables|/Script/AudioSynesthesia.ConstantQNRT|GetSettings (Variables|Default|GetQNRT_Constant))) 1))
    (bind _returnvalue (AddComponent|AddStaticMeshComponent false (Math|Transform|MakeTransform (Math|Vector|MakeVector (* (Variables|Default|GetPadding) _index) 0.0 0.0) "0.000000,0.000000,90.000000" (Variables|Default|GetScale))))
    (Utilities|Array|Add (Variables|Default|GetMeshComponents) _returnvalue)
    (Rendering|Material|SetVectorParameterValueonMaterials _returnvalue "EmissiveColor" (.OutItem (Utilities|Array|Random (Variables|Default|GetColors))))))